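; SignPost_BP is an interactable sign that shows its name and text in the game's dialogue box.
; On Interact, it writes SignName and SignText to the message box widget held by ThirdPersonGameMode and shows it.
; The box hides after a fixed delay, or when an overlap with the sign's Box component ends as something moves away.
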(event OnComponentEndOverlap(box)
  (params (OverlappedComponent :type Primitive%20Component%20Object%20Reference) (OtherActor :type Actor%20Object%20Reference) (OtherComp :type Primitive%20Component%20Object%20Reference) (OtherBodyIndex :type Integer))
  ;[1 1 1] Removes Dialogue when moving away
  (bind _asthird_person_game_mode (Utilities|Casting|CastToThirdPersonGameMode (Game|GetGameMode)))
  (Widget|SetVisibility (Variables|/Game/AlexT/DialogueStuff/UserInterface/HeadsUpDisplay.HeadsUpDisplay_C|GetDialogueBox (Variables|/Game/ThirdPersonBP/Blueprints/ThirdPersonGameMode.ThirdPersonGameMode_C|GetMessageBoxRef _asthird_person_game_mode)) "Hidden"))

(event EventInteract
  ;[1 1 1] Comment
  (bind _asthird_person_game_mode (Utilities|Casting|CastToThirdPersonGameMode (Game|GetGameMode)))
  (Variables|/Game/AlexT/DialogueStuff/UserInterface/DialogueBox.DialogueBox_C|SetSpeaker (Variables|/Game/AlexT/DialogueStuff/UserInterface/HeadsUpDisplay.HeadsUpDisplay_C|GetDialogueBox (Variables|/Game/ThirdPersonBP/Blueprints/ThirdPersonGameMode.ThirdPersonGameMode_C|GetMessageBoxRef _asthird_person_game_mode)) (Variables|Default|GetSignName))
  (Variables|/Game/AlexT/DialogueStuff/UserInterface/DialogueBox.DialogueBox_C|SetDialogueText (Variables|/Game/AlexT/DialogueStuff/UserInterface/HeadsUpDisplay.HeadsUpDisplay_C|GetDialogueBox (Variables|/Game/ThirdPersonBP/Blueprints/ThirdPersonGameMode.ThirdPersonGameMode_C|GetMessageBoxRef _asthird_person_game_mode)) (Variables|Default|GetSignText))
  (Widget|SetVisibility (Variables|/Game/AlexT/DialogueStuff/UserInterface/HeadsUpDisplay.HeadsUpDisplay_C|GetDialogueBox (Variables|/Game/ThirdPersonBP/Blueprints/ThirdPersonGameMode.ThirdPersonGameMode_C|GetMessageBoxRef _asthird_person_game_mode)) "Visible")
  (Utilities|FlowControl|Delay 5.0)
  (Widget|SetVisibility (Variables|/Game/AlexT/DialogueStuff/UserInterface/HeadsUpDisplay.HeadsUpDisplay_C|GetDialogueBox (Variables|/Game/ThirdPersonBP/Blueprints/ThirdPersonGameMode.ThirdPersonGameMode_C|GetMessageBoxRef _asthird_person_game_mode)) "Hidden"))

(fn ConstructionScript)